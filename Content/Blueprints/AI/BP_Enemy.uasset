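; BP_Enemy is an AI-controlled enemy that reacts to damage and death through its health component.
; It caches its AIC_Enemy controller on BeginPlay and unpossesses itself when health runs out.
; While alive, hits from EM_MagicProjectile set the controller's ReceivingDamage flag and report an AI perception damage event at the projectile owner's location, identifying that owner as instigator.
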(event OnHealthChangeDelegate(HealthComponent)
  (params (HealthComponent :type EM%20Health%20Component%20Object%20Reference) (DamagedActor :type Actor%20Object%20Reference) (Damage :type Float%20%28single-precision%29) (DamageType :type Damage%20Type%20Object%20Reference) (InstigatedBy :type Controller%20Object%20Reference) (DamageCauser :type Actor%20Object%20Reference))
  (if (Class|EMHealthComponent|IsDead HealthComponent)
    (Pawn|UnPossess (Pawn|GetController))
    (else
      (bind _asem_magic_projectile (Utilities|Casting|CastToEM_MagicProjectile DamageCauser))
      (Utilities|FlowControl|Sequence
        (:then_0
          (bind _aicontroller (Variables|Default|GetAIController)
            (:then
              (Variables|/Script/Arkde_RoomPuzzleGame.EM_AIController|SetbReceivingDamage _aicontroller true))
            (:else)))
        (:then_1
          (Class|AISenseDamage|ReportDamageEvent self (Components|GetOwner _asem_magic_projectile) Damage (Transformation|GetActorLocation (Components|GetOwner _asem_magic_projectile))))))))

(event EventBeginPlay
  (bind _asaic_enemy (Utilities|Casting|CastToAIC_Enemy (Pawn|GetController)))
  (Variables|Default|SetAIController _asaic_enemy))

(event Collision|EventActorBeginOverlap
  (params (OtherActor :type Actor%20Object%20Reference)))

(event EventTick
  (params (DeltaSeconds :type Float%20%28single-precision%29)))

(fn ConstructionScript)